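; Player character Blueprint for the Jester, creating the HUD, options menu and inventory widget, and unlocking doors with small or boss keys.
; Tick shows the game-over screen and destroys the actor at zero health, otherwise turns full bleed, burn and poison meters into status flags and syncs effect and key visibility.
; Hardcoded keys raise, lower or cleanse those meters.
; Throwable functions swap the held mesh and set aim and throw flags, respecting locks.
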(event `Key|Escape`
  (params (Key :type "Key Structure" :default "AnyKey"))
  ;[1 1 1] Open Options
  (:`Pressed`
    ;;[1 1 1] Check Platform
    (bind _returnvalue (`GameplayStatics.GetPlatformName`))
    (if (not (`KismetStringLibrary.EqualEqual_StrStr` _returnvalue "Windows"))
      (bind _returnvalue_2 (`|CreateWidget` "/Game/Game/Assets/Blueprints/Player/Options_Menu.Options_Menu_C"))
      (`UserWidget.AddToViewport` (stale `Key|Tab` _returnvalue_2) 0 :!label _label)
      (`UserWidget.AddToViewport` _returnvalue_2 0))))

(event `Key|B`
  (params (Key :type "Key Structure" :default "AnyKey"))
  (bind _doortounlock (`self.DoorToUnlock`))
  (bind _numsmallkeys (`self.NUMSmallKeys`))
  ;[1 1 1] Unlock Door
  (:`Pressed`
    (`/Engine/EditorBlueprintResources/StandardMacros.IsValid` _doortounlock
      (:`Is Valid`
        (if (`/Game/Game/Assets/SceneAssets/L00Dungeon/LockedDoor/ABP_LockedDoor.CanUnlock` _doortounlock)
          (if (`|EnumEquality` (`/Game/Game/Assets/SceneAssets/L00Dungeon/LockedDoor/ABP_LockedDoor.TPYEOF Door` _doortounlock) "NewEnumerator0")
            (if (> (`self.NUMSmallKeys`) 0)
              (`/Game/Game/Assets/SceneAssets/L00Dungeon/LockedDoor/ABP_LockedDoor.UnlockDoor` (`self.DoorToUnlock`))
              (set `self.NUMSmallKeys` (- _numsmallkeys 1))
              (if (< _numsmallkeys 1)
                (set `self.Has00SmallKey00` false)
                (else
                  (set `self.Has00SmallKey00` true))))
            (elif (`self.Has00BossKey`)
              (`/Game/Game/Assets/SceneAssets/L00Dungeon/LockedDoor/ABP_LockedDoor.UnlockDoor` (`self.DoorToUnlock`)))))))))

(event `Key|Tab`
  (params (Key :type "Key Structure" :default "AnyKey"))
  ;[1 1 1] Open Options
  (:`Pressed`
    ;;[1 1 1] Check Platform
    (bind _returnvalue (`GameplayStatics.GetPlatformName`))
    (if (`KismetStringLibrary.EqualEqual_StrStr` _returnvalue "Windows")
      (bind _returnvalue_2 (`|CreateWidget` "/Game/Game/Assets/Blueprints/Player/Options_Menu.Options_Menu_C"))
      (goto _label))))

(event `self.ReceiveBeginPlay`
  (bind _returnvalue (`GameplayStatics.GetPlayerController` 0))
  ;[1 1 1] BeginPlay: Create HUD, Save a reference, Add it to viewport, set input mode
  (set `PlayerController.bShowMouseCursor` true _returnvalue)
  (bind _returnvalue_2 (`|CreateWidget` "/Game/UI/Jester/UI_JESTER_HUD.UI_JESTER_HUD_C"))
  (bind _output_get (set `self.REF_InGameHUD` _returnvalue_2))
  (`UserWidget.AddToViewport` _output_get 0)
  (`WidgetBlueprintLibrary.SetInputMode_GameAndUIEx` _returnvalue _output_get "DoNotLock" false))

(event `Key|O`
  (params (Key :type "Key Structure" :default "AnyKey"))
  ;[1 1 1] BLEED
  (:`Pressed`
    (set `self.SE_BLEED_BuildUp` (+ (`self.SE_BLEED_BuildUp`) -14.2))))

(event `Key|I`
  (params (Key :type "Key Structure" :default "AnyKey"))
  ;[1 1 1] BLEED
  ;;[1 1 1] UP
  (:`Pressed`
    (set `self.SE_BLEED_BuildUp` (+ (`self.SE_BLEED_BuildUp`) 14.2))))

(event `Key|Comma`
  (params (Key :type "Key Structure" :default "AnyKey"))
  ;[1 1 1] BLEED
  ;;[1 1 1] UP
  (:`Pressed`
    (set `self.SE_POISON_BuildUp` (+ (`self.SE_POISON_BuildUp`) 14.2))))

(event `Key|Period`
  (params (Key :type "Key Structure" :default "AnyKey"))
  ;[1 1 1] BLEED
  (:`Pressed`
    (set `self.SE_POISON_BuildUp` (+ (`self.SE_POISON_BuildUp`) -14.2))))

(event `Key|P`
  (params (Key :type "Key Structure" :default "AnyKey"))
  ;[1 1 1] BLEED
  ;;[1 1 1] CLEANSE BLEED
  (:`Pressed`
    (set `self.IsBLEEDING` false)
    (set `self.SE_BLEED_BuildUp` 0.0)))

(event `Key|P`
  (params (Key :type "Key Structure" :default "AnyKey"))
  ;[1 1 1] BLEED
  ;;[1 1 1] CLEANSE BLEED
  (:`Pressed`
    (set `self.SE_POISON_BuildUp` 0.0)
    (set `self.IsPOISONED` false)))

(event `Key|L`
  (params (Key :type "Key Structure" :default "AnyKey"))
  ;[1 1 1] BURN
  (:`Pressed`
    (set `self.SE_BURN_BuildUp` (+ (`self.SE_BURN_BuildUp`) -14.2))))

(event `Key|K`
  (params (Key :type "Key Structure" :default "AnyKey"))
  ;[1 1 1] BURN
  ;;[1 1 1] UP
  (:`Pressed`
    (set `self.SE_BURN_BuildUp` (+ (`self.SE_BURN_BuildUp`) 14.2))))

(event `Key|P`
  (params (Key :type "Key Structure" :default "AnyKey"))
  ;[1 1 1] BURN
  ;;[1 1 1] CLEANSE BLEED
  (:`Pressed`
    (set `self.SE_BURN_BuildUp` 0.0)
    (set `self.IsBURNING` false)))

(event `self.ReceiveTick`
  (params (DeltaSeconds :type "Float (single-precision)"))
  (bind _has00smallkey00 (`self.Has00SmallKey00`))
  ;[1 1 1] Is he dead?
  (if (<= (`self.HealthCurrent`) 0.0)
    ;[1 1 1] Add Game Over Screen
    (bind _returnvalue (`|CreateWidget` "/Game/UI/Jester/GameOverScreen.GameOverScreen_C"))
    (bind _output_get (set `self.GOScreenRef` _returnvalue))
    (`UserWidget.AddToViewport` _output_get 0)
    (`WidgetBlueprintLibrary.SetInputMode_UIOnlyEx` (`GameplayStatics.GetPlayerController` 0) _output_get)
    (`self.K2_DestroyActor`)
    (else
      ;[1 1 1] IsBLEEDING
      (if (>= (`self.SE_BLEED_BuildUp`) (`self.SE_BLEED_MaxAmount`))
        (`SceneComponent.SetVisibility` (`self.PS_SE_BLEEDING`) true true)
        (set `self.SE_BLEED_BuildUp` 0.0)
        (set `self.IsBLEEDING` true))
      ;[1 1 1] isBURNING
      (if (>= (`self.SE_BURN_BuildUp`) (`self.SE_BURN_MaxAmount`))
        (`SceneComponent.SetVisibility` (`self.PS_SE_BURNING`) true true)
        (set `self.SE_BURN_BuildUp` 0.0)
        (set `self.IsBURNING` true))
      ;[1 1 1] IsPOISONED
      (if (>= (`self.SE_POISON_BuildUp`) (`self.SE_POISON_MaxAmount`))
        (`SceneComponent.SetVisibility` (`self.PS_SE_POISONED`) true true)
        (set `self.SE_POISON_BuildUp` 0.0)
        (set `self.IsPOISONED` true))
      ;[1 1 1] VisBlood
      (if (and (not (`self.IsBLEEDING`)) (== (`self.SE_BLEED_BuildUp`) 0.0))
        (`SceneComponent.SetVisibility` (`self.PS_SE_BLEEDING`) false false))
      ;[1 1 1] VisBurn
      (if (and (not (`self.IsBURNING`)) (== (`self.SE_BURN_BuildUp`) 0.0))
        (`SceneComponent.SetVisibility` (`self.PS_SE_BURNING`) false false))
      ;[1 1 1] VisPoison
      (if (and (not (`self.IsPOISONED`)) (== (`self.SE_POISON_BuildUp`) 0.0))
        (`SceneComponent.SetVisibility` (`self.PS_SE_POISONED`) false false))
      ;[1 1 1] VisKey
      (`SceneComponent.SetVisibility` (`self.SM_00_SmallKey00`) _has00smallkey00 false)
      (`SceneComponent.SetVisibility` (`self.PS_SmallKey`) _has00smallkey00 false))))

(event `self.OpenInventory`
  (bind _ref_ui_inventory (`self.REF_UI_Inventory`))
  ;[1 1 1] Inventory
  (if (`self.HasOpenedInventory`)
    (set `self.HasOpenedInventory` false)
    (`Widget.RemoveFromParent` _ref_ui_inventory)
    (else
      (set `self.HasOpenedInventory` true)
      (if (not (`self.Has_REF_UI_Inventory`))
        (bind _returnvalue (`|CreateWidget` "/Game/UI/Jester/UI_JESTER_Inventory.UI_JESTER_Inventory_C"))
        (bind _output_get (set `self.REF_UI_Inventory` _returnvalue))
        (set `self.Has_REF_UI_Inventory` true)
        (`/Game/UI/Jester/UI_JESTER_Inventory.SetREF_Jester` _output_get self))
      (`UserWidget.AddToViewport` _ref_ui_inventory 0)
      (`KismetSystemLibrary.PrintString` "OpenInventory"))))

(event `self.AimCurrentThrowable`
  (set `self.IsAimingThrowable` true))

(event `self.ThrowCurrentThrowable`
  ;[1 1 1] Throw item
  (set `self.IsAimingThrowable` false)
  (if (`|EnumEquality` (`self.CurrentThrowable`) "NONE")
    (`KismetSystemLibrary.PrintString` "NoThrowable")
    (elif (`self.IsThrowLocked`)
      (`KismetSystemLibrary.PrintString` "ThrowLocked" true true (struct :`R` 1.0 :`G` 0.03 :`B` 0.03 :`A` 1.0))
      (else
        (set `self.IsThrowingSomething` true)))))

(fn `EquipThrowable`
  (params (`Type of Throwable` :type "ETYPEOF_Throwable Enum"))
  (bind _stmesh_throwable (`self.STMESH_Throwable`))
  (if (not (`self.IsThrowableSwapLocked`))
    (bind _output_get (set `self.CurrentThrowable` `Type of Throwable`))
    (switch `ETYPEOF_Throwable` _output_get
      (:`KNIFE`
        (`StaticMeshComponent.SetStaticMesh` _stmesh_throwable "/Game/Game/Assets/Throwables/ThrowingKnife/STMESH_ThrowKnife.STMESH_ThrowKnife"))
      (:`NONE`
        (`StaticMeshComponent.SetStaticMesh` _stmesh_throwable null)))))

(fn `GetDoorToUnlock`
  (params (LockedDoor :type "/Game/Game/Assets/SceneAssets/L00Dungeon/LockedDoor/ABP_LockedDoor Object Reference"))
  (set `self.DoorToUnlock` LockedDoor))

(fn `PickupSmallKey`
  (`/Engine/EditorBlueprintResources/StandardMacros.IncrementInt` (`self.NUMSmallKeys`)))

(fn `UserConstructionScript`)