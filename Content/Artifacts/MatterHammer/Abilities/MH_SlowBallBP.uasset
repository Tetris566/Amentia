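; MH_SlowBallBP is a Matter Hammer projectile that damages the enemies it overlaps.
; On BeginPlay a charge above one scales both mesh size and damage, and the ball destroys itself after a fixed delay.
; Mesh overlaps ignore player-tagged actors, damage either of two enemy base classes through their respective damage calls and destroy the ball.
; Any other overlap zeroes its velocity, leaving it in place.
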(event `self.ReceiveBeginPlay`
  (bind _mesh (`self.Mesh`))
  (bind _ballcharge (`self.BallCharge`))
  (if (> (`self.BallCharge`) 1.0)
    (`SceneComponent.SetWorldScale3D` _mesh (* (`SceneComponent.K2_GetComponentScale` _mesh) _ballcharge))
    (set `self.Damage` (* _ballcharge (`self.Damage`))))
  (`KismetSystemLibrary.Delay` 6.0)
  (`self.K2_DestroyActor`))

(event `self.Mesh.OnComponentBeginOverlap`
  (params (OverlappedComponent :type "PrimitiveComponent Object Reference") (OtherActor :type "Actor Object Reference") (OtherComp :type "PrimitiveComponent Object Reference") (OtherBodyIndex :type Integer) (bFromSweep :type Boolean) (SweepResult :type "HitResult Structure (by ref)"))
  (bind _damage (`self.Damage`))
  (if (not (`self.ActorHasTag` OtherActor "Player"))
    (bind _asenemy_base (cast `/Game/NPCs/Enemies/Enemy_Base` OtherActor)
      (:`then`
        (`/Game/NPCs/Enemies/Enemy_Base.ReceiveDamage` _asenemy_base _damage)
        (`self.K2_DestroyActor`))
      (:`CastFailed`
        (bind _askoa_base_enemy_character (cast `KOA_BASE_EnemyCharacter` OtherActor)
          (:`then`
            (`GameplayStatics.ApplyDamage` _askoa_base_enemy_character _damage)
            (`self.K2_DestroyActor`))
          (:`CastFailed`
            (`ProjectileMovementComponent.SetVelocityInLocalSpace` (`self.ProjectileMovement`) (0.0 0.0 0.0))))))))

(fn `UserConstructionScript`)