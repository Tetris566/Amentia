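; MH_PillarBP is a short-lived pillar actor for a Matter Hammer artifact ability that rises out of its spawn point.
; On BeginPlay it records its starting height and destroys itself after two seconds.
; Each tick it teleports upward at a constant speed until it reaches a fixed offset above that starting height.
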(event `self.ReceiveBeginPlay`
  (bind (_returnvalue_x _returnvalue_y _returnvalue_z) (`KismetMathLibrary.BreakVector` (`self.K2_GetActorLocation`)))
  (set `self.StartingHeight` _returnvalue_z)
  (`KismetSystemLibrary.Delay` 2.0)
  (`self.K2_DestroyActor`))

(event `self.ReceiveTick`
  (params (DeltaSeconds :type "Float (single-precision)"))
  (bind (_returnvalue_x _returnvalue_y _returnvalue_z) (`KismetMathLibrary.BreakVector` (`self.K2_GetActorLocation`)))
  (bind (_returnvalue_x_2 _returnvalue_y_2 _returnvalue_z_2) (`KismetMathLibrary.BreakVector` (`self.K2_GetActorLocation`)))
  (if (< _returnvalue_z_2 (+ (`self.StartingHeight`) 300.0))
    (`self.K2_SetActorLocation` (`KismetMathLibrary.MakeVector` _returnvalue_x _returnvalue_y (+ _returnvalue_z (* DeltaSeconds 1000.0))) false true)))

(fn `UserConstructionScript`)