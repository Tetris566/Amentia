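; BP_SpikePit is a dungeon spike pit hazard that damages characters standing in it.
; Begin and end overlap events toggle a single Touching flag, and Tick reads the actor from the begin-overlap event while that flag is set.
; A cast chain routes damage to the Jester player, cat guard or base enemy, spawning a blood spurt at the victim.
; Damage applies every frame, unscaled by delta time.
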(event `self.ReceiveActorBeginOverlap`
  (params (OtherActor :type "Actor Object Reference"))
  (set `self.Touching` true))

(event `self.ReceiveActorEndOverlap`
  (params (OtherActor :type "Actor Object Reference"))
  (set `self.Touching` false))

(event `self.ReceiveTick`
  (params (DeltaSeconds :type "Float (single-precision)"))
  (if (`self.Touching`)
    (bind _aspcbp_jester (cast `/Game/Jester/Blueprints/PCBP_Jester` (stale `self.ReceiveActorBeginOverlap` OtherActor))
      (:`then`
        (`KOA_PROTO_Character.DamagePlayer` _aspcbp_jester 0.5)
        (bind _returnvalue (`self.K2_GetActorLocation` (stale `self.ReceiveActorBeginOverlap` OtherActor)))
        (`GameplayStatics.SpawnEmitterAtLocation` "/Game/BloodFX/BloodSpurt.BloodSpurt" _returnvalue))
      (:`CastFailed`
        (bind _asbp_enpc_cat_guard (cast `/Game/NPCs/Enemies/CatGuard/BP_ENPC_CatGuard` (stale `self.ReceiveActorBeginOverlap` OtherActor))
          (:`then`
            (`KOA_BASE_EnemyCharacter.ReceiveDamage` _asbp_enpc_cat_guard 0.5)
            (`GameplayStatics.SpawnEmitterAtLocation` "/Game/BloodFX/BloodSpurt.BloodSpurt" _returnvalue))
          (:`CastFailed`
            (bind _asenemy_base (cast `/Game/NPCs/Enemies/Enemy_Base` (stale `self.ReceiveActorBeginOverlap` OtherActor)))
            (`/Game/NPCs/Enemies/Enemy_Base.ReceiveDamage` _asenemy_base 0.5)
            (`GameplayStatics.SpawnEmitterAtLocation` "/Game/BloodFX/BloodSpurt.BloodSpurt" _returnvalue)))))))

(fn `UserConstructionScript`)