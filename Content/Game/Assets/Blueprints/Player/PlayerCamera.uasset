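; Side-view player camera that becomes the view target at BeginPlay and follows the player in the YZ plane.
; Each Tick, CameraState selects one of four modes: target lock with zoom, smoothed follow (also the default), velocity-based look-ahead, or box camera.
; Lock mode frames the midpoint between player and CameraTarget, deriving depth from that midpoint and MaxDepth.
; Box mode overwrites CameraTarget, stepping sideways faster the farther the player leaves a horizontal dead zone.
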(event `self.ReceiveTick`
  (params (DeltaSeconds :type "Float (single-precision)"))
  (bind (_returnvalue_x _returnvalue_y _returnvalue_z) (`KismetMathLibrary.BreakVector` (`self.K2_GetActorLocation`)))
  (bind (_returnvalue_x_2 _returnvalue_y_2) (`KismetMathLibrary.BreakVector` (`self.K2_GetActorLocation`)))
  (bind (_returnvalue_x_3 _returnvalue_y_3) (`KismetMathLibrary.BreakVector` (`self.K2_GetActorLocation`)))
  (bind (_returnvalue_x_4 _returnvalue_y_4) (`KismetMathLibrary.BreakVector` (`self.K2_GetActorLocation`)))
  (bind (_returnvalue_x_5 _returnvalue_y_5) (`KismetMathLibrary.BreakVector` (`self.K2_GetActorLocation`)))
  (bind _returnvalue (`GameplayStatics.GetPlayerCharacter` 0))
  (bind _returnvalue_2 (`GameplayStatics.GetWorldDeltaSeconds`))
  (bind _cammovespeed (`self.CamMoveSpeed`))
  (bind (_returnvalue_x_6 _returnvalue_y_6 _returnvalue_z_2) (`KismetMathLibrary.BreakVector` (`self.K2_GetActorLocation` _returnvalue)))
  (bind (_returnvalue_x_7 _returnvalue_y_7 _returnvalue_z_3) (`KismetMathLibrary.BreakVector` (`self.K2_GetActorLocation` (`GameplayStatics.GetPlayerCharacter` 0))))
  (bind (_returnvalue_x_8 _returnvalue_y_8 _returnvalue_z_4) (`KismetMathLibrary.BreakVector` (`self.K2_GetActorLocation` (`GameplayStatics.GetPlayerCharacter` 0))))
  (bind (_returnvalue_x_9 _returnvalue_y_9 _returnvalue_z_5) (`KismetMathLibrary.BreakVector` (`self.GetVelocity` _returnvalue)))
  (bind _returnvalue_3 (* 600.0 _returnvalue_2))
  (bind _returnvalue_4 (* 900.0 _returnvalue_2))
  (bind _returnvalue_5 (- _returnvalue_y_8 _returnvalue_y_5))
  (bind _returnvalue_6 (- _returnvalue_y_8 _returnvalue_y_5))
  (bind _returnvalue_7 (+ _returnvalue_z_4 100.0))
  (bind (_returnvalue_x_10 _returnvalue_y_10) (`KismetMathLibrary.BreakVector2D` (`KismetMathLibrary.Vector2DInterpTo` (`KismetMathLibrary.MakeVector2D` _returnvalue_y _returnvalue_z) (`KismetMathLibrary.MakeVector2D` _returnvalue_y_7 (+ _returnvalue_z_3 100.0)) DeltaSeconds (`self.CamSpeed`))))
  (bind (_returnvalue_x_11 _returnvalue_y_11 _returnvalue_z_6) (`KismetMathLibrary.BreakVector` (* (+ (`self.CameraTarget`) (`self.K2_GetActorLocation` (`GameplayStatics.GetPlayerCharacter` 0))) 0.5)))
  (bind (_returnvalue_x_12 _returnvalue_y_12) (`KismetMathLibrary.BreakVector` (+ (`KismetMathLibrary.MakeVector` 0.0 (* _returnvalue_y_9 0.3) (* _returnvalue_z_5 0.1)) (`self.K2_GetActorLocation` _returnvalue))))
  (bind _returnvalue_8 (+ _returnvalue_y_11 -100.0))
  (bind _returnvalue_9 (+ _returnvalue_z_6 100.0))
  (bind _returnvalue_10 (* (`KismetMathLibrary.Abs` (* (+ _returnvalue_y_11 _returnvalue_z_6) 1.2)) -1.0))
  ;[1 1 1] Camera Switch
  (switch `int` (`self.CameraState`) :!label _label
    (:`Default`
      ;[1 1 1] Interpolation
      (`self.K2_SetActorLocation` (`KismetMathLibrary.MakeVector` -700.0 _returnvalue_x_10 _returnvalue_y_10) :!label _label_2))
    (:`0`
      ;[1 1 1] Lock and Zoom
      (if (< (`self.MaxDepth`) _returnvalue_10)
        (`self.K2_SetActorLocation` (`KismetMathLibrary.MakeVector` (`self.MaxDepth`) _returnvalue_8 _returnvalue_9))
        (else
          (`self.K2_SetActorLocation` (`KismetMathLibrary.MakeVector` _returnvalue_10 _returnvalue_8 _returnvalue_9)))))
    (:`1`
      (goto _label_2))
    (:`2`
      ;[1 1 1] Momentum/Predictive
      (`self.K2_SetActorLocation` (`KismetMathLibrary.MakeVector` -700.0 _returnvalue_y_12 _returnvalue_z_2)))
    (:`3`
      ;[1 1 1] Box Cam
      (if (> _returnvalue_6 300.0)
        (if (> _returnvalue_5 400.0)
          (set `self.CamMoveSpeed` _returnvalue_4)
          (else
            (set `self.CamMoveSpeed` _returnvalue_3)))
        (set `self.CameraTarget` (`KismetMathLibrary.MakeVector` -700.0 (+ _returnvalue_y_3 _cammovespeed) _returnvalue_7))
        (elif (< _returnvalue_6 -300.0)
          (if (< _returnvalue_5 -400.0)
            (set `self.CamMoveSpeed` _returnvalue_4)
            (else
              (set `self.CamMoveSpeed` _returnvalue_3)))
          (set `self.CameraTarget` (`KismetMathLibrary.MakeVector` -700.0 (- _returnvalue_y_4 _cammovespeed) _returnvalue_7))
          (else
            (set `self.CameraTarget` (`KismetMathLibrary.MakeVector` -700.0 _returnvalue_y_2 _returnvalue_7)))))
      (`self.K2_SetActorLocation` (`KismetMathLibrary.VInterpTo` (`self.K2_GetActorLocation`) (`self.CameraTarget`) (`GameplayStatics.GetWorldDeltaSeconds`) (`self.InterpolationSpeed`))))))

(event `self.ReceiveBeginPlay`
  (bind (_returnvalue_x _returnvalue_y) (`KismetMathLibrary.BreakVector` (`self.K2_GetActorLocation`)))
  ;[1 1 1] Camera Switch
  (set `self.bFindCameraComponentWhenViewTarget` false)
  (`PlayerController.SetViewTargetWithBlend` (`GameplayStatics.GetPlayerController` 0) self 0.0 "VTBlend_Linear" 0.0 false)
  (`self.K2_SetActorLocation` (`KismetMathLibrary.MakeVector` -700.0 _returnvalue_y 200.0))
  (goto _label))

(fn `UserConstructionScript`)