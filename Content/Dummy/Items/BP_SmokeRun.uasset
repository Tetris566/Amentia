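; BP_SmokeRun is an actor that moves its particle system, by its name a smoke effect, around a looping path of relative locations.
; Tick disables itself, then MoveComponentTo moves the component to the current MovePoints entry over a fixed duration with zero relative rotation.
; The index then advances, wrapping at the array's end, and Tick is re-enabled, so the latent move and tick toggle act as the loop.
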(event `self.ReceiveTick`
  (params (DeltaSeconds :type "Float (single-precision)"))
  (`self.SetActorTickEnabled` false)
  (`KismetSystemLibrary.MoveComponentTo` (`self.ParticleSystem`) (`KismetArrayLibrary.Array_Get` (`self.Move Points`) (`self.index`)) (struct) false false 3.0)
  (`/Engine/EditorBlueprintResources/StandardMacros.IncrementInt` (`self.index`)
    (:`  `
      (if (>= (`self.index`) (`KismetArrayLibrary.Array_Length` (`self.Move Points`)))
        (set `self.index` 0))
      (`self.SetActorTickEnabled` true))))

(fn `UserConstructionScript`)