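; Dummy enemy character base that tracks health and exercises sections of a test animation montage.
; Health starts at MaxHealth and drops with any damage, with helper functions for the dead check and health percentage.
; BeginPlay plays two delayed Kick sections, while Tick calls Att every frame, followed by Kick and Roll through latent Delays.
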(event `self.ReceiveBeginPlay`
  (set `self.Health` (`self.Max Health`))
  (`KismetSystemLibrary.Delay` 1.5)
  (`self.PlayAnimMontage` "/Game/Enemy/Dummy/test.test" 1.0 "Kick")
  (`KismetSystemLibrary.Delay` 4.0)
  (`self.PlayAnimMontage` "/Game/Enemy/Dummy/test.test" 1.0 "Kick"))

(event `self.ReceiveTick`
  (params (DeltaSeconds :type "Float (single-precision)"))
  (`self.PlayAnimMontage` "/Game/Enemy/Dummy/test.test" 1.0 "Att")
  (`KismetSystemLibrary.Delay` 0.25)
  (`self.PlayAnimMontage` "/Game/Enemy/Dummy/test.test" 1.0 "Kick")
  (`KismetSystemLibrary.Delay` 0.4)
  (`self.PlayAnimMontage` "/Game/Enemy/Dummy/test.test" 1.0 "Roll"))

(event `self.ReceiveAnyDamage`
  (params (Damage :type "Float (single-precision)") (DamageType :type "DamageType Object Reference") (InstigatedBy :type "Controller Object Reference") (DamageCauser :type "Actor Object Reference"))
  (set `self.Health` (- (`self.Health`) Damage)))

(fn `Convert Health to Percent`
  (returns (ReturnValue :type "Float (double-precision)"))
  (return (/ (`self.Health`) (`self.Max Health`))))

(fn `Is Dead`
  (returns (ReturnValue :type Boolean))
  (return (<= (`self.Health`) 0.0)))

(fn `UserConstructionScript`)