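; Base enemy Blueprint that provides a helper for turning the enemy to face a world position along the Y axis.
; RotateToFacePos checks whether the position lies on the positive or negative Y side of the actor and snaps yaw to the matching perpendicular heading, preserving roll and pitch.
; The event graph and construction script contain no active logic.
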(fn `RotateToFacePos`
  (params (Position :type "Vector Structure"))
  (bind _returnvalue (`self.K2_GetActorRotation`))
  (if (<= 0.0 (.y (- Position (`self.K2_GetActorLocation`))))
    (`self.K2_SetActorRotation` (`KismetMathLibrary.MakeRotator` (.roll _returnvalue) (.pitch _returnvalue) 90.0))
    (else
      (`self.K2_SetActorRotation` (`KismetMathLibrary.MakeRotator` (.roll _returnvalue) (.pitch _returnvalue) -90.0)))))

(fn `UserConstructionScript`)