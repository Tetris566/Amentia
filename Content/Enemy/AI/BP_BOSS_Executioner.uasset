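; Executioner boss enemy character with a health-bar widget shown when the fight starts and an event that unlocks the Jester's artifact storm.
; Tick calls NextStage until the boss is dead and not falling, then disables capsule collision, removes the UI and starts one-shot death effects.
; Death restores the non-flashing material, then a timeline drives a dynamic material's dissolve before destroying the actor.
; Hits make its capsule ignore other enemy characters while moving.
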(event `self.ReceiveTick`
  (params (DeltaSeconds :type "Float (single-precision)"))
  ;[1 1 1] TICK
  (if (and (not (`NavMovementComponent.IsFalling` (`self.CharacterMovement`))) (`self.Is Dead`))
    (`PrimitiveComponent.SetCollisionEnabled` (`self.CapsuleComponent`) "NoCollision")
    (`Widget.RemoveFromParent` (`self.REF_UI`))
    (if (`self.Is Dead`)
      (if (not (`self.HasStoppedFlashing`))
        (set `self.HasStoppedFlashing` true)
        (`self.StopFlashing`))
      (if (not (`self.HasDissolved`))
        (set `self.HasDissolved` true)
        (`KismetSystemLibrary.Delay` 2.0)
        (`self.EVENT_Dissolve`)))
    (else
      ;[1 1 1] Set Stage
      (`self.Next Stage`))))

(event `self.ReceiveBeginPlay`
  (bind _mesh (`self.Mesh`))
  (bind _returnvalue (`PrimitiveComponent.GetMaterial` _mesh 0))
  ;[1 1 1] EVENT: Begin Play
  (`parent.ReceiveBeginPlay`)
  (`KismetSystemLibrary.PrintString` (`KismetSystemLibrary.GetDisplayName` _returnvalue))
  (bind _returnvalue_2 (`PrimitiveComponent.CreateDynamicMaterialInstance` _mesh 0 _returnvalue))
  (set `self.DissolveMaterial` _returnvalue_2)
  (bind _returnvalue_3 (`|CreateWidget` "/Game/UI/NPC/WBP_UI_BOSS_HPBard.WBP_UI_BOSS_HPBard_C"))
  (bind _output_get (set `self.REF_UI` _returnvalue_3))
  (`/Game/UI/NPC/WBP_UI_BOSS_HPBard.SetREF_BOSS` _output_get null)
  (bind _aspcbp_jester (cast `/Game/Jester/Blueprints/PCBP_Jester` (`GameplayStatics.GetPlayerCharacter` 0)))
  (set `self.REF_Jester` _aspcbp_jester))

(event `EVENT_StartBossFight`
  ;[1 1 1] EVENT: Start Boss Fight
  (`UserWidget.AddToViewport` (stale `self.ReceiveBeginPlay` _output_get) 0))

(event `EVENT_Dissolve`
  ;[1 1 1] Dissolve and Delete Boss
  (`PrimitiveComponent.SetMaterial` (`Character.Mesh` (`self.REF_BOSS_Executioner`)) 0 (`self.DissolveMaterial`))
  (bind (_direction _dissolve) (`Timeline|DissolveTimeline`)
    (:`Update`
      (`MaterialInstanceDynamic.SetScalarParameterValue` (`self.DissolveMaterial`) "DissolveAmount" _dissolve))
    (:`Finished`
      (`KismetSystemLibrary.Delay` 2.0)
      (`self.K2_DestroyActor` (`self.REF_BOSS_Executioner`)))))

(event `EVENT_UnlockBloodStorm`
  ;[1 1 1] EVENT: UNLOCK BLOOD STORM
  (bind _aspcbp_jester (cast `/Game/Jester/Blueprints/PCBP_Jester` (`GameplayStatics.GetPlayerCharacter` 0)))
  (set `KOA_BASE_Artifact.IsArtifactStormUnlocked` true (`KOA_PROTO_Character.GetCurrArtifactReference` _aspcbp_jester)))

(event `self.ReceiveHit`
  (params (MyComp :type "PrimitiveComponent Object Reference") (Other :type "Actor Object Reference") (OtherComp :type "PrimitiveComponent Object Reference") (bSelfMoved :type Boolean) (HitLocation :type "Vector Structure") (HitNormal :type "Vector Structure") (NormalImpulse :type "Vector Structure") (Hit :type "HitResult Structure (by ref)"))
  (bind _askoa_base_enemy_character (cast `KOA_BASE_EnemyCharacter` Other))
  (`PrimitiveComponent.IgnoreActorWhenMoving` (`self.CapsuleComponent`) _askoa_base_enemy_character true))

(fn `GetStage`
  (returns (currentStage :type Integer))
  (return (`self.currentStage`)))

(fn `StartFlashing`
  (`PrimitiveComponent.SetMaterial` (`self.Mesh`) 0 "/Game/NPCs/BOSS/Executioner/Model/Guard_02_Flashing.Guard_02_Flashing"))

(fn `StopFlashing`
  (`PrimitiveComponent.SetMaterial` (`self.Mesh`) 0 "/Game/NPCs/BOSS/Executioner/Model/Guard_02.Guard_02"))

(fn `UserConstructionScript`
  (set `self.HasDissolved` false)
  (set `self.HasStoppedFlashing` false))