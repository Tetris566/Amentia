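; Base boss enemy that owns a boss HP bar widget, tracks fight stages and dissolves on death.
; The HP bar is created on BeginPlay, along with a cached Jester player reference, and shown when the boss fight starts.
; Damage updates the stage from health-percent thresholds, or on death removes the bar and runs a timeline-driven dynamic-material dissolve before destroying the actor.
; ToggleFlash swaps the mesh between normal and flashing materials.
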(event `self.ReceiveBeginPlay`
  (`parent.ReceiveBeginPlay`)
  ;[1 1 1] EVENT: Begin Play
  (bind _returnvalue (`|CreateWidget` "/Game/Enemy/AI/WBP_UI_BOSS_HPBard.WBP_UI_BOSS_HPBard_C"))
  (bind _output_get (set `self.REF_UI` _returnvalue))
  (`/Game/Enemy/AI/WBP_UI_BOSS_HPBard.SetREF_BOSS` _output_get self)
  (bind _aspcbp_jester (cast `/Game/Jester/Blueprints/PCBP_Jester` (`GameplayStatics.GetPlayerCharacter` 0)))
  (set `self.REF_Jester` _aspcbp_jester))

(event `EVENT_StartBossFight`
  ;[1 1 1] EVENT: Start Boss Fight
  (`UserWidget.AddToViewport` (`self.REF_UI`) 0))

(event `EVENT_Dissolve`
  ;[1 1 1] Dissolve and Delete Boss
  (`self.Setup Disolve`)
  (bind (_direction _dissolve) (`Timeline|Timeline_0`)
    (:`Update`
      (`MaterialInstanceDynamic.SetScalarParameterValue` (`self.DissolveMaterial`) "DissolveAmount" _dissolve))
    (:`Finished`
      (`KismetSystemLibrary.Delay` 2.0)
      (`self.K2_DestroyActor`))))

(event `self.ReceiveAnyDamage`
  (params (Damage :type "Float (single-precision)") (DamageType :type "DamageType Object Reference") (InstigatedBy :type "Controller Object Reference") (DamageCauser :type "Actor Object Reference"))
  ;[1 1 1] Dissolve or Set Stage
  (`parent.ReceiveAnyDamage` Damage DamageType InstigatedBy DamageCauser)
  (if (`self.Is Dead`)
    (`Widget.RemoveFromParent` (`self.REF_UI`))
    (`self.EVENT_Dissolve`)
    (else
      (`self.Setup Stage`))))

(event `Setup Disolve`
  (bind _mesh (`self.Mesh`))
  (bind _returnvalue (`PrimitiveComponent.CreateDynamicMaterialInstance` _mesh 0 "/Game/NPCs/BOSS/Executioner/Model/MATI_ExecutionerDissolve.MATI_ExecutionerDissolve"))
  (bind _output_get (set `self.DissolveMaterial` _returnvalue))
  (`MaterialInstanceDynamic.SetTextureParameterValue` _output_get "BaseColorTexture" (`self.Mat_Normal`))
  (`PrimitiveComponent.SetMaterial` _mesh 0 _output_get))

(fn `Setup Stage`
  (locals (StageThresholds :type "Array of Float (double-precision)") (tmpStage :type Integer))
  (for (_array_element _array_index) (`local.StageThresholds`)
    (if (<= (`self.Convert Health to Percent`) _array_element)
      (set `local.tmpStage` (+ _array_index 1))))
  (set `self.Current Stage` (`local.tmpStage`)))

(fn `Toggle Flash`
  (params (`Is Flashing` :type Boolean :default false))
  (bind _mesh (`self.Mesh`))
  (if `Is Flashing`
    (`PrimitiveComponent.SetMaterial` _mesh 0 "/Game/NPCs/BOSS/Executioner/Model/Guard_02_Flashing.Guard_02_Flashing")
    (else
      (`PrimitiveComponent.SetMaterial` _mesh 0 "/Game/NPCs/BOSS/Executioner/Model/Guard_02.Guard_02"))))

(fn `UserConstructionScript`
  (`parent.UserConstructionScript`))