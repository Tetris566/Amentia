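; AI controller for the Executioner boss that starts and seeds its behavior tree.
; On BeginPlay it applies the Executioner blackboard, sets defaults (chasing state, player character as target, wall kick allowed), then runs the behavior tree.
; EnableWallKicking sets the wall-kick flag back to true; nothing in this file calls it or clears the flag.
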(event EventBeginPlay
  (Class|AIController|UseBlackboard "/Game/NPCs/BOSS/Executioner/AI/BB_ExecutionerBlackboard.BB_ExecutionerBlackboard")
  (CallFunction|SetBlackboardDefaults)
  (AI|RunBehaviorTree "/Game/NPCs/BOSS/Executioner/AI/BehaviorTrees/BT_ExecutionerBehavior.BT_ExecutionerBehavior"))

(event EventTick
  (params (DeltaSeconds :type Float%20%28single-precision%29)))

(fn ConstructionScript)

(fn SetBlackboardDefaults
  (bind _returnvalue (AI|GetBlackboard 0))
  (AI|Components|Blackboard|SetValueasEnum _returnvalue (LocalVariables|GetBBN_CurrentState) (LocalVariables|GetChasing))
  (AI|Components|Blackboard|SetValueasObject _returnvalue (LocalVariables|GetBBN_TargetActor) (Game|GetPlayerCharacter 0))
  (AI|Components|Blackboard|SetValueasBool _returnvalue (LocalVariables|GetBBN_CanKickWall) true))

(fn EnableWallKicking
  (AI|Components|Blackboard|SetValueasBool (AI|GetBlackboard 0) (LocalVariables|GetBBN_CanKickWall) true))